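; BP_PickupWeapon is a world weapon pickup that characters can take, and whose reserve ammo can also be drawn separately.
; Interact passes the weapon class, location, ammo and ammo type to the character's SpawnWeapon, then destroys the pickup.
; An interface getter exposes the ammo struct, and IFTakeReserveAmmo subtracts from any positive reserve without clamping.
; Taking ammo also pops the pickup object with a randomized upward impulse and plays a shotgun ammo sound.
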(event `/Game/MyProject/Interfaces/BPI_Interact.Interact`
  (params (CharacterPickingUp :type "/Game/MyProject/Character/BP_ThirdPersonCharacter Object Reference"))
  (`/Game/MyProject/Character/BP_ThirdPersonCharacter.Spawn Weapon` CharacterPickingUp (`self.Weapon To Spawn`) (`self.K2_GetActorLocation`) (`self.Ammo`) (`self.Ammo Type`))
  (`self.K2_DestroyActor`))

(event `/Game/MyProject/Interfaces/BPI_WeaponPickup.IF_TakeReserveAmmo`
  (params (`Ammo Taken` :type Integer))
  (bind (_ammotype _ammoindex _reserveammo _maxreserveammo _has_) (break `/Game/MyProject/Props/Weapons/Ammo/Struct_Ammo` (`self.Ammo Type`)))
  (if (> _reserveammo 0)
    (set `self.Ammo Type` (make `/Game/MyProject/Props/Weapons/Ammo/Struct_Ammo` _ammotype _ammoindex (- _reserveammo `Ammo Taken`) _maxreserveammo _has_))
    (`PrimitiveComponent.AddImpulse` (`self.PickupObject`) (`KismetMathLibrary.MakeVector` (`KismetMathLibrary.RandomFloatInRange` -25.0 25.0) (`KismetMathLibrary.RandomFloatInRange` -25.0 25.0) (`KismetMathLibrary.RandomFloatInRange` 125.0 150.0)) "None" false)
    (`GameplayStatics.PlaySoundAtLocation` "/Game/MilitaryWeapSilver/Sound/Shotgun/Cues/Shotgun_AmmoPickup_Cue.Shotgun_AmmoPickup_Cue" (`self.K2_GetActorLocation`) (struct) 1.0 1.0 0.0 null null null null)))

(fn `IF_GetAmmoType`
  (returns (AmmoType :type "/Game/MyProject/Props/Weapons/Ammo/Struct_Ammo Structure"))
  (return (`self.Ammo Type`)))

(fn `UserConstructionScript`
  (`parent.UserConstructionScript`))