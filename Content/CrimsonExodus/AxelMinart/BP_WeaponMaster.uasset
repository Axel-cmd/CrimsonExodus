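; BP_WeaponMaster is a weapon Blueprint that provides the cosmetic effects of firing an assault rifle.
; Its Fire event spawns a muzzle flash and plays the rifle sound at the WeaponModel's muzzle socket.
; It also spawns an ammo actor at the AmmoEject socket and kicks it along that socket's right vector with a mass-independent impulse.
; The graph contains no trace, damage or ammo-count logic.
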(event `/Game/MyProject/Interfaces/BPI_Fire.Fire`
  (bind _weaponmodel (`self.WeaponModel`))
  (bind (_returnvalue_location _returnvalue_rotation) (`KismetMathLibrary.BreakTransform` (`SceneComponent.GetSocketTransform` (`self.WeaponModel`) "muzzle" "RTS_World")))
  (bind _returnvalue (`SceneComponent.GetSocketRotation` _weaponmodel "AmmoEject"))
  (`GameplayStatics.SpawnEmitterAtLocation` "/Game/MilitaryWeapDark/FX/P_AssaultRifle_MuzzleFlash.P_AssaultRifle_MuzzleFlash" _returnvalue_location _returnvalue_rotation)
  (`GameplayStatics.PlaySoundAtLocation` "/Game/MilitaryWeapSilver/Sound/Rifle/Cues/RifleA_Fire_Cue.RifleA_Fire_Cue" _returnvalue_location (struct) 1.0 1.0 0.0 null null null null)
  (bind _returnvalue_2 (`|SpawnActorFromClass` "/Game/MyProject/Props/Weapons/AssaultRifle/BP_AssaultRifleB_Ammo.BP_AssaultRifleB_Ammo_C" (`KismetMathLibrary.MakeTransform` (`SceneComponent.GetSocketLocation` _weaponmodel "AmmoEject") _returnvalue) "Undefined" "MultiplyWithRoot" null null))
  (`PrimitiveComponent.AddImpulse` (`/Game/MyProject/Props/Weapons/AssaultRifle/BP_AssaultRifleB_Ammo.Ammo` _returnvalue_2) (* (`KismetMathLibrary.GetRightVector` _returnvalue) 100.0) "None" true))

(fn `UserConstructionScript`)