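; BP_Character is a character Blueprint for Crimson Exodus that tracks health, death and attack state.
; UpdateHP adds a signed delta to HealthPoint without clamping, then calls UpdateIsDead, which sets IsDead at zero or below.
; Getters expose IsDead and IsAttacking, though nothing here sets IsAttacking.
; TriggerDeath and TriggerAttack are empty, and reaching zero health does not call TriggerDeath.
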(event `UpdateIsDead`
  ;[1 1 1] check if is dead
  (if (<= (`self.HealthPoint`) 0)
    (set `self.IsDead` true)
    (else
      (set `self.IsDead` false))))

(fn `getIsAttacking`
  (returns (IsAttacking :type Boolean))
  (return (`self.IsAttacking`)))

(fn `getIsDead`
  (returns (IsDead :type Boolean))
  (return (`self.IsDead`)))

(fn `triggerAttack`)

(fn `TriggerDeath`)

(fn `Update HP`
  (params (Delta :type Integer))
  (returns (newHP :type Integer))
  ;[0.008192 0 0.09896] Update HP
  (bind _output_get (set `self.HealthPoint` (+ Delta (`self.HealthPoint`))))
  (`self.UpdateIsDead`)
  (return _output_get))

(fn `UserConstructionScript`)