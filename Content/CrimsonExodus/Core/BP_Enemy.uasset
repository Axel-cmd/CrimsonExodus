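; BP_Enemy is an AI enemy that deals contact damage to BP_Hero and can be killed.
; Overlapping PlayerDamagingBox hits the hero immediately, then a looping timer derived from EnemyDPS repeats DamageHero until the hero leaves.
; When damage kills it, it detaches its controller, disables capsule collision and clears the timer.
; TriggerDeath, called after the death animation, notifies the game mode to decrement the enemy count and destroys the actor.
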(event `/Game/CrimsonExodus/Core/BPI_Damageable.AffectHealth`
  (params (Delta :type Integer))
  ;[1 1 1] Manage damage taken
  (if (not (`self.IsDead`))
    (`self.Update HP` Delta)
    (if (`self.IsDead`)
      (`self.DetachFromControllerPendingDestroy`)
      (`PrimitiveComponent.SetCollisionEnabled` (`self.CapsuleComponent`) "NoCollision")
      (`KismetSystemLibrary.K2_ClearAndInvalidateTimerHandle` (`self.DamageTimer`)))))

(event `self.TriggerDeath`
  ;[1 1 1] called when ai death animation finished
  (`parent.TriggerDeath`)
  (if (`self.IsDead`)
    (message `/Game/CrimsonExodus/Core/BPI_GameMode_MP.DecrementEnemyCount` (`GameplayStatics.GetGameMode`))
    (`self.K2_DestroyActor`)))

(event `self.PlayerDamagingBox.OnComponentBeginOverlap`
  (params (OverlappedComponent :type "PrimitiveComponent Object Reference") (OtherActor :type "Actor Object Reference") (OtherComp :type "PrimitiveComponent Object Reference") (OtherBodyIndex :type Integer) (bFromSweep :type Boolean) (SweepResult :type "HitResult Structure (by ref)"))
  ;[1 1 1] Does damage to hero
  (bind _asbp_hero (cast `/Game/CrimsonExodus/Core/BP_Hero` OtherActor))
  (set `self.Hero` _asbp_hero)
  (`self.DamageHero`)
  (bind _returnvalue (`KismetSystemLibrary.K2_SetTimerDelegate` (`|CreateDelegate` :!event `DamageHero`) (/ 1.0 (`self.EnemyDPS`)) true))
  (set `self.DamageTimer` _returnvalue))

(event `DamageHero`
  ;[1 1 1] Does damage to hero
  (set `self.IsAttacking` true)
  (`/Game/CrimsonExodus/Core/BPI_Damageable.AffectHealth` (`self.Hero`) (`self.DamageAmount`)))

(event `self.PlayerDamagingBox.OnComponentEndOverlap`
  (params (OverlappedComponent :type "PrimitiveComponent Object Reference") (OtherActor :type "Actor Object Reference") (OtherComp :type "PrimitiveComponent Object Reference") (OtherBodyIndex :type Integer))
  ;[1 1 1] Stop dealing damage when hero is far
  (if (== OtherActor (`self.Hero`))
    (set `self.IsAttacking` false)
    (`KismetSystemLibrary.K2_ClearAndInvalidateTimerHandle` (`self.DamageTimer`))))

(fn `UserConstructionScript`
  (`parent.UserConstructionScript`))