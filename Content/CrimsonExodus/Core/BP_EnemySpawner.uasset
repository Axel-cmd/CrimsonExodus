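; Enemy spawner actor that places BP_Enemy AI pawns at random points inside its SpawnZone box.
; It registers itself with the game mode on BeginPlay and exposes a SpawnOneEnemy event.
; Each spawn request first asks the game mode for permission, then reports back to increment the enemy count.
; All game mode communication goes through message calls, without casting to a specific class.
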(event `self.ReceiveBeginPlay`
  ;[1 1 1] Control spawner
  (message `/Game/CrimsonExodus/Core/BPI_GameMode_MP.RegisterSpawner` (`GameplayStatics.GetGameMode`) self))

(event `SpawnOneEnemy`
  (bind _spawnzone (`self.SpawnZone`))
  ;[1 1 1] Spawn an enemy in a random location
  (bind _result (message `/Game/CrimsonExodus/Core/BPI_GameMode_MP.CanSpawnOneEnemy` (`GameplayStatics.GetGameMode`)))
  (if _result
    (`AIBlueprintHelperLibrary.SpawnAIFromClass` "/Game/CrimsonExodus/Core/BP_Enemy.BP_Enemy_C" null (`KismetMathLibrary.RandomPointInBoundingBox` (`SceneComponent.K2_GetComponentLocation` _spawnzone) (`BoxComponent.GetScaledBoxExtent` _spawnzone)) (struct) false null)
    (message `/Game/CrimsonExodus/Core/BPI_GameMode_MP.IncrementEnemyCount` (`GameplayStatics.GetGameMode`))))

(fn `UserConstructionScript`)