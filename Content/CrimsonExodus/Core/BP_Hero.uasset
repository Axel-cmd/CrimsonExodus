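; BP_Hero is the player-controlled top-down hero, handling movement, mouse aiming, damage and death.
; Enhanced Input drives world-axis movement and turns the control rotation toward the cursor, found by intersecting a deprojected mouse ray with a horizontal plane at the hero's height.
; Health changes go through UpdateHP, disabling input on death.
; It registers its spawn transform with BP_Gamemode, which TriggerDeath asks to respawn the player before destroying the actor.
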(event `self.ReceiveBeginPlay`
  (`|ExecutionSequence`
    (:`then_0`
      (`EnhancedInputSubsystemInterface.AddMappingContext` (pcsubsystem `EnhancedInputLocalPlayerSubsystem` (`GameplayStatics.GetPlayerController` 0)) "/Game/CrimsonExodus/Core/inputs/IMP_TopDown.IMP_TopDown" 0 (struct)))
    (:`then_1`
      ;[1 1 1] send start positionfor respawn
      (bind _asbp_gamemode (cast `/Game/CrimsonExodus/Core/BP_Gamemode` (`GameplayStatics.GetGameMode`)))
      (bind _output_get (set `self.Gamemode` _asbp_gamemode))
      (`/Game/CrimsonExodus/Core/BP_Gamemode.setPlayerSpawnTransform` _output_get (`self.GetTransform`)))))

(event `EnhancedInput|/Game/CrimsonExodus/Core/inputs/INP_MoveAround`
  (params (ActionValue :type "Vector2D Structure") (ElapsedSeconds :type "Float (double-precision)") (TriggeredSeconds :type "Float (double-precision)") (InputAction :type "InputAction Object Reference" :default "/Game/CrimsonExodus/Core/inputs/INP_MoveAround.INP_MoveAround"))
  (:`Triggered`
    (`self.AddMovementInput` (0.0 1.0 0.0) ActionValue_X)
    (`self.AddMovementInput` (1.0 0.0 0.0) ActionValue_Y)))

(event `EnhancedInput|/Game/CrimsonExodus/Core/inputs/INP_LookAround`
  (params (ActionValue :type Boolean) (ElapsedSeconds :type "Float (double-precision)") (TriggeredSeconds :type "Float (double-precision)") (InputAction :type "InputAction Object Reference" :default "/Game/CrimsonExodus/Core/inputs/INP_LookAround.INP_LookAround"))
  (bind _returnvalue (`GameplayStatics.GetPlayerController` 0))
  (bind _returnvalue_2 (`GameplayStatics.GetPlayerController` 0))
  (bind _returnvalue_3 (`self.K2_GetActorLocation`))
  (bind (_locationx _locationy) (`PlayerController.GetMousePosition` _returnvalue))
  (bind (_worldposition _worlddirection) (`GameplayStatics.DeprojectScreenToWorld` _returnvalue (`KismetMathLibrary.MakeVector2D` _locationx _locationy)))
  (:`Triggered`
    (`Controller.SetControlRotation` _returnvalue (`KismetMathLibrary.FindLookAtRotation` _returnvalue_3 (`.Intersection` (`KismetMathLibrary.LinePlaneIntersection_OriginNormal` _worldposition (+ _worldposition (* _worlddirection 5000.0)) _returnvalue_3 (0.0 0.0 1.0))))))
  (:`Started`
    (set `PlayerController.bShowMouseCursor` true _returnvalue_2)
    (`WidgetBlueprintLibrary.SetInputMode_GameOnly` _returnvalue_2 :!label _label))
  (:`Completed`
    (set `PlayerController.bShowMouseCursor` false _returnvalue_2)
    (goto _label)))

(event `/Game/CrimsonExodus/Core/BPI_Damageable.AffectHealth`
  (params (Delta :type Integer))
  ;[1 1 1] Manage damage to hero
  (if (not (`self.IsDead`))
    (bind _newhp (`self.Update HP` Delta))
    (`KismetSystemLibrary.PrintString` (`KismetStringLibrary.Concat_StrStr` "HP Player = " (`KismetStringLibrary.Conv_IntToString` _newhp)))
    (if (`self.IsDead`)
      (`self.DisableInput` (`GameplayStatics.GetPlayerController` 0)))))

(event `self.TriggerDeath`
  ;[1 1 1] Called func aftter death animation
  (`parent.TriggerDeath`)
  (if (`self.IsDead`)
    (`/Game/CrimsonExodus/Core/BP_Gamemode.RespawnPlayer` (`self.Gamemode`))
    (`self.K2_DestroyActor`)))

(fn `UserConstructionScript`
  (`parent.UserConstructionScript`))